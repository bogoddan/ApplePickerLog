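; BP_ApplePickerGM is the Apple Picker game mode, which so far only sets up the HUD.
; On BeginPlay, CreateHUD adds a WB_HUD widget to the viewport and fills it with apples collected and high score from BP_ApplePickerGS.
; SpawnBaskets and DeleteBasket are empty stubs, and the only SpawnBaskets call is never reached.
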(event `self.ReceiveBeginPlay`
  (`self.CreateHUD`))

(fn `CreateHUD`
  (bind _returnvalue (`|CreateWidget` "/Game/UI/WB_HUD.WB_HUD_C"))
  (`UserWidget.AddToViewport` _returnvalue 0)
  (bind _output_get (set `self.HUD` _returnvalue))
  (bind _asbp_apple_picker_gs (cast `/Game/Blueprints/BP_ApplePickerGS` (`GameplayStatics.GetGameState`)))
  (`/Game/UI/WB_HUD.UpdateHUD` _output_get (`/Game/Blueprints/BP_ApplePickerGS.ApplesCollected` _asbp_apple_picker_gs) (`/Game/Blueprints/BP_ApplePickerGS.HighScore` _asbp_apple_picker_gs))
  (`KismetSystemLibrary.PrintText` "HUD Created"))

(fn `DeleteBasket`)

(fn `SpawnBaskets`)

(fn `UserConstructionScript`)