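; Game state Blueprint for the apple picker game, tracking apples collected and a persistent high score.
; On BeginPlay it loads the high score from a save slot, if one exists, and broadcasts it.
; Each collection event increments the C++-backed count, fires a dispatcher and, when the count reaches the high score, immediately saves it via BP_SaveGameHS and broadcasts it.
; It also relays log records through a refresh dispatcher.
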(event `self.ReceiveBeginPlay`
  (`self.LoadSavedGameIfExist`))

(event `self.UpdateApplesCollected`
  (`self.IncrementApplesCollected`))

(event `self.RefreshLogs`
  (params (LogRecords :type "Array of String (by ref)"))
  (`self.RefreshLogsDispatcher` LogRecords))

(fn `IncrementApplesCollected`
  (returns (ApplesCollected :type Integer))
  (bind _result (`/Engine/EditorBlueprintResources/StandardMacros.IncrementInt` (`self.ApplesCollected_cpp`))
    (:`  `
      (`self.AppleCollectedDispatcher` _result)
      (`self.UpdateHighScore`)
      (return _result))))

(fn `LoadSavedGameIfExist`
  (bind _savehs (`self.SaveHS`))
  (bind _returnvalue (`GameplayStatics.DoesSaveGameExist` _savehs))
  (if _returnvalue
    (bind _returnvalue_2 (`GameplayStatics.LoadGameFromSlot` _savehs))
    (bind _output_get (set `self.GameSaverHS` _returnvalue_2))
    (bind _asbp_save_game_hs (cast `/Game/Blueprints/BP_SaveGameHS` _output_get))
    (bind _output_get_2 (set `self.HighScore` (`/Game/Blueprints/BP_SaveGameHS.HighScore` _asbp_save_game_hs)))
    (`self.HighScoreDispatcher` _output_get_2)))

(fn `UpdateHighScore`
  (bind _applescollected_cpp (`self.ApplesCollected_cpp`))
  (bind _savehs (`self.SaveHS`))
  (bind _savehs_2 (`self.SaveHS`))
  (bind _gamesaverhs (`self.GameSaverHS`))
  (bind _highscore (`self.HighScore`))
  (if (>= _applescollected_cpp _highscore)
    (set `self.HighScore` _applescollected_cpp)
    (bind _returnvalue (`GameplayStatics.DoesSaveGameExist` _savehs))
    (if _returnvalue
      (bind _returnvalue_2 (`GameplayStatics.LoadGameFromSlot` _savehs))
      (bind _output_get (set `self.GameSaverHS` _returnvalue_2))
      (bind _asbp_save_game_hs (cast `/Game/Blueprints/BP_SaveGameHS` _output_get))
      (bind _output_get_2 (set `/Game/Blueprints/BP_SaveGameHS.HighScore` _highscore _asbp_save_game_hs))
      (`GameplayStatics.SaveGameToSlot` _gamesaverhs _savehs_2)
      (`self.HighScoreDispatcher` _output_get_2)
      (else
        (bind _returnvalue_3 (`GameplayStatics.CreateSaveGameObject` "/Game/Blueprints/BP_SaveGameHS.BP_SaveGameHS_C"))
        (bind _output_get_3 (set `self.GameSaverHS` _returnvalue_3))
        (bind _asbp_save_game_hs_2 (cast `/Game/Blueprints/BP_SaveGameHS` _output_get_3))
        (bind _output_get_4 (set `/Game/Blueprints/BP_SaveGameHS.HighScore` _highscore _asbp_save_game_hs_2))
        (`GameplayStatics.SaveGameToSlot` _gamesaverhs _savehs_2)
        (`self.HighScoreDispatcher` _output_get_4)))))

(fn `UserConstructionScript`)