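; BP_AppleTree is an apple tree actor with Blueprint functions for side-to-side movement along Y within a game field.
; InitializeEdgesBP sets edges around the tree's position, and IsTimeToChangeDirectionBP flags turns at those edges or randomly, weighted by delta time.
; MoveTreeBP currently adds zero offset, while direction change and apple dropping are unfinished stubs with unwired nodes.
; The event graph is empty, so nothing here calls these functions.
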(event `self.ReceiveBeginPlay`)

(fn `Change Direction_BP`)

(fn `DropApple1`)

(fn `Initialize Edges_BP`
  (bind _gamefieldsize (`self.GameFieldSize`))
  (bind _y (.y (`self.K2_GetActorLocation`)))
  (set `self.LeftEdge` (- _y _gamefieldsize))
  (set `self.RightEdge` (+ _y _gamefieldsize)))

(fn `IsTimeToChangeDirection_BP`
  (params (DeltaSeconds :type "Float (double-precision)") (`CurrentY OfTree` :type "Float (double-precision)"))
  (returns (ChangeDirection :type Boolean))
  (return (or (or (<= `CurrentY OfTree` (`self.LeftEdge`)) (>= `CurrentY OfTree` (`self.RightEdge`))) (`KismetMathLibrary.RandomBoolWithWeight` (* DeltaSeconds (`self.chanceToChangeDirections`))))))

(fn `MoveTree_BP`
  (params (DeltaSeconds :type "Float (double-precision)"))
  (returns (`Corrent Y Of Tree` :type "Float (double-precision)"))
  (bind _returnvalue (+ (.y (`self.K2_GetActorLocation`)) (* DeltaSeconds 0.0)))
  (`self.K2_SetActorLocation` (`KismetMathLibrary.MakeVector` (.x (`self.K2_GetActorLocation`)) _returnvalue (.z (`self.K2_GetActorLocation`))))
  (return _returnvalue))

(fn `UserConstructionScript`)